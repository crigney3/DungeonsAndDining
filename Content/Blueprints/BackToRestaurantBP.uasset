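; BackToRestaurantBP is a world trigger that shows a "Back to Restaurant (Press F)" prompt for returning to the restaurant.
; On BeginPlay it caches the player character, hides the widget component and restyles its reused ContainerOpenWidget text.
; Sphere overlaps toggle prompt visibility, while Box overlaps set the CollidingWithGoHome flag, both without filtering the overlapping actor.
; The F input and the travel itself are not handled here.
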(event `self.ReceiveBeginPlay`
  (bind _returnvalue (`GameplayStatics.GetActorOfClass` "/Game/Blueprints/BarbarianThirdPersonCharacter.BarbarianThirdPersonCharacter_C"))
  (set `self.PlayerRef` _returnvalue)
  (`SceneComponent.SetVisibility` (`self.GoHomeWidget`) false false)
  (bind _ascontainer_open_widget (cast `/Game/Blueprints/ContainerOpenWidget` (`WidgetComponent.GetUserWidgetObject` (`self.GoHomeWidget`))))
  (`/Game/Blueprints/ContainerOpenWidget.SetNewText` _ascontainer_open_widget "Back to Restaurant (Press F)")
  (bind _opentext (`/Game/Blueprints/ContainerOpenWidget.OpenText` _ascontainer_open_widget))
  (bind (_fontobject _fontmaterial _outlinesettings _typefacefontname _size _letterspacing _skewamount) (break `SlateFontInfo` (`TextBlock.Font` _opentext)))
  (`TextBlock.SetFont` _opentext (make `SlateFontInfo` _fontobject _fontmaterial _outlinesettings _typefacefontname 64.0 _letterspacing _skewamount))
  (`TextBlock.SetAutoWrapText` _opentext true))

(event `self.ReceiveTick`
  (params (DeltaSeconds :type "Float (single-precision)")))

(event `self.Sphere.OnComponentBeginOverlap`
  (params (OverlappedComponent :type "PrimitiveComponent Object Reference") (OtherActor :type "Actor Object Reference") (OtherComp :type "PrimitiveComponent Object Reference") (OtherBodyIndex :type Integer) (bFromSweep :type Boolean) (SweepResult :type "HitResult Structure (by ref)"))
  (`SceneComponent.SetVisibility` (`self.GoHomeWidget`) true false))

(event `self.Sphere.OnComponentEndOverlap`
  (params (OverlappedComponent :type "PrimitiveComponent Object Reference") (OtherActor :type "Actor Object Reference") (OtherComp :type "PrimitiveComponent Object Reference") (OtherBodyIndex :type Integer))
  (`SceneComponent.SetVisibility` (`self.GoHomeWidget`) false false))

(event `self.Box.OnComponentBeginOverlap`
  (params (OverlappedComponent :type "PrimitiveComponent Object Reference") (OtherActor :type "Actor Object Reference") (OtherComp :type "PrimitiveComponent Object Reference") (OtherBodyIndex :type Integer) (bFromSweep :type Boolean) (SweepResult :type "HitResult Structure (by ref)"))
  (set `self.CollidingWithGoHome` true))

(event `self.Box.OnComponentEndOverlap`
  (params (OverlappedComponent :type "PrimitiveComponent Object Reference") (OtherActor :type "Actor Object Reference") (OtherComp :type "PrimitiveComponent Object Reference") (OtherBodyIndex :type Integer))
  (set `self.CollidingWithGoHome` false))

(fn `UserConstructionScript`)