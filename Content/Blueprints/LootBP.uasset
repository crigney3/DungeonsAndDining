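; Loot pickup actor with a configurable mesh and a rarity-based outline overlay material set in the construction script.
; A range sphere tracks the player, either auto-collecting or toggling a pickup widget according to PickupType; one type ignores overlaps.
; PlayerPickupLoot guards against repeat pickup and passes the loot to every BarbarianThirdPersonCharacter.
; PhaseOutAndDestroy applies a rarity-tinted dissolve material and sets a delayed lifespan.
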(event `self.ReceiveBeginPlay`
  (`SceneComponent.SetVisibility` (`self.PickupWidget`) false false)
  (`SphereComponent.SetSphereRadius` (`self.PickupRangeCollisionSphere`) (`self.PickupRange`) true))

(event `self.PickupRangeCollisionSphere.OnComponentBeginOverlap`
  (params (OverlappedComponent :type "PrimitiveComponent Object Reference") (OtherActor :type "Actor Object Reference") (OtherComp :type "PrimitiveComponent Object Reference") (OtherBodyIndex :type Integer) (bFromSweep :type Boolean) (SweepResult :type "HitResult Structure (by ref)"))
  (if (`|EnumInequality` (`self.Pickup Type`) "NewEnumerator2")
    (if (== OtherActor (`GameplayStatics.GetPlayerCharacter` 0))
      (set `self.PlayerInPickupRange` true)
      (if (`|EnumEquality` (`self.Pickup Type`) "NewEnumerator0")
        (`KismetSystemLibrary.PrintString` "auto-pickup loot")
        (`self.PlayerPickupLoot`)
        (else
          (`self.UpdateWidgetVisiblity`))))))

(event `self.PickupRangeCollisionSphere.OnComponentEndOverlap`
  (params (OverlappedComponent :type "PrimitiveComponent Object Reference") (OtherActor :type "Actor Object Reference") (OtherComp :type "PrimitiveComponent Object Reference") (OtherBodyIndex :type Integer))
  (if (`|EnumInequality` (`self.Pickup Type`) "NewEnumerator2")
    (if (== OtherActor (`GameplayStatics.GetPlayerCharacter` 0))
      (set `self.PlayerInPickupRange` false)
      (`self.UpdateWidgetVisiblity`))))

(fn `GetRarityMaterialColor`
  (returns (`Rarity Material Color` :type "LinearColor Structure"))
  (locals (CommonRarityColor :type "LinearColor Structure" :default (struct :`R` 0.94902 :`G` 1.0 :`B` 0.956863 :`A` 1.0)) (UncommonRarityColor :type "LinearColor Structure" :default (struct :`R` 0.007843 :`G` 1.0 :`B` 0.156863 :`A` 1.0)) (RareRarityColor :type "LinearColor Structure" :default (struct :`R` 0.84 :`G` 3.63 :`B` 100.0 :`A` 1.0)) (EpicRarityColor :type "LinearColor Structure" :default (struct :`R` 0.937255 :`B` 1.0 :`A` 1.0)) (LegendaryRarityColor :type "LinearColor Structure" :default (struct :`R` 10.0 :`G` 5.2 :`A` 1.0)) (MythicRarityColor :type "LinearColor Structure" :default (struct :`R` 10.0 :`G` 0.286275 :`A` 1.0)))
  (switch `/Game/Blueprints/LootRarity` (`self.Loot Rarity`)
    (:`NewEnumerator0`
      (return (`local.CommonRarityColor`)))
    (:`NewEnumerator1`
      (return (`local.UncommonRarityColor`)))
    (:`NewEnumerator2`
      (return (`local.RareRarityColor`)))
    (:`NewEnumerator3`
      (return (`local.EpicRarityColor`)))
    (:`NewEnumerator4`
      (return (`local.LegendaryRarityColor`)))
    (:`NewEnumerator5`
      (return (`local.MythicRarityColor`)))))

(fn `PhaseOutAndDestroy`
  (bind _returnvalue (`KismetMaterialLibrary.CreateDynamicMaterialInstance` "/Game/Materials/DissolveInstance3.DissolveInstance3"))
  (bind _rarity_material_color (`self.GetRarityMaterialColor`))
  (`MaterialInstanceDynamic.SetVectorParameterValue` _returnvalue "SecondBurnColor" _rarity_material_color)
  (`PrimitiveComponent.SetMaterial` (`self.LootMesh`) 0 _returnvalue)
  (`self.SetLifeSpan` (`self.DestructionDelay`)))

(fn `PlayerPickupLoot`
  (if (`self.ItemPickedUp`)
    _
    (elif (`self.PlayerInPickupRange`)
      (set `self.ItemPickedUp` true)
      (bind _outactors (`GameplayStatics.GetAllActorsOfClass` "/Game/Blueprints/BarbarianThirdPersonCharacter.BarbarianThirdPersonCharacter_C"))
      (for _array_element _outactors
        (`/Game/Blueprints/BarbarianThirdPersonCharacter.PickupItem` _array_element self)
        (`self.PhaseOutAndDestroy`)))))

(fn `UpdateWidgetVisiblity`
  (`SceneComponent.SetVisibility` (`self.PickupWidget`) (`self.PlayerInPickupRange`) false))

(fn `UserConstructionScript`
  (locals (OverlayMaterialInstance :type "MaterialInstance Object Reference"))
  (`StaticMeshComponent.SetStaticMesh` (`self.LootMesh`) (`self.CustomLootMesh`))
  (switch `/Game/Blueprints/LootRarity` (`self.Loot Rarity`)
    (:`NewEnumerator0`
      (set `local.OverlayMaterialInstance` "/Game/Materials/CommonLootOutline_MI.CommonLootOutline_MI"))
    (:`NewEnumerator1`
      (set `local.OverlayMaterialInstance` "/Game/Materials/UncommonLootOutline_MI.UncommonLootOutline_MI"))
    (:`NewEnumerator2`
      (set `local.OverlayMaterialInstance` "/Game/Materials/RareLootOutline_MI.RareLootOutline_MI"))
    (:`NewEnumerator3`
      (set `local.OverlayMaterialInstance` "/Game/Materials/EpicLootOutline_MI.EpicLootOutline_MI"))
    (:`NewEnumerator4`
      (set `local.OverlayMaterialInstance` "/Game/Materials/LegendaryLootOutline_MI.LegendaryLootOutline_MI"))
    (:`NewEnumerator5`
      (set `local.OverlayMaterialInstance` "/Game/Materials/MythicLootOutline_MI.MythicLootOutline_MI")))
  (`MeshComponent.SetOverlayMaterial` (`self.LootMesh`) (`local.OverlayMaterialInstance`))
  (`SphereComponent.SetSphereRadius` (`self.PickupRangeCollisionSphere`) (`self.PickupRange`) true))