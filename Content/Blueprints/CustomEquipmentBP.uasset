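; Equipment display actor that shows a configurable mesh with a rarity-colored loot outline and a weapon trail.
; UpdateEquipmentAttributes sets the mesh, scale and rotation, then picks the outline overlay material by rarity.
; For socketed meshes, it centers the WeaponTrail between BottomSocket and TopSocket, aligns it, derives ribbon width from their scaled distance and assigns a rarity trail material.
; The construction script applies defaults and hides the trail, which SetTrailVisibility toggles.
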(fn `GetWeaponTrailMaterialInstance`
  (params (WeaponRarity :type "/Game/Blueprints/LootRarity Enum" :default "NewEnumerator0"))
  (returns (TrailMaterialInstance :type "MaterialInstance Object Reference"))
  (switch `/Game/Blueprints/LootRarity` WeaponRarity
    (:`NewEnumerator0`
      (return "/Game/Materials/CommonWeaponTrail_MI.CommonWeaponTrail_MI"))
    (:`NewEnumerator1`
      (return "/Game/Materials/UncommonWeaponTrail_MI.UncommonWeaponTrail_MI"))
    (:`NewEnumerator2`
      (return "/Game/Materials/RareWeaponTrail_MI.RareWeaponTrail_MI"))
    (:`NewEnumerator3`
      (return "/Game/Materials/EpicWeaponTrail_MI.EpicWeaponTrail_MI"))
    (:`NewEnumerator4`
      (return "/Game/Materials/LegendaryWeaponTrail_MI.LegendaryWeaponTrail_MI"))
    (:`NewEnumerator5`
      (return "/Game/Materials/MythicWeaponTrail_MI.MythicWeaponTrail_MI"))))

(fn `SetTrailVisibility`
  (params (IsVisible :type Boolean))
  (`SceneComponent.SetVisibility` (`self.WeaponTrail`) IsVisible false))

(fn `Update Equipment Attributes`
  (params (EquipmentMesh :type "StaticMesh Object Reference") (EquipmentRarity :type "/Game/Blueprints/LootRarity Enum" :default "NewEnumerator0") (DisplayScale :type "Vector Structure") (TrailDisplayScale :type "Vector Structure") (DisplayRotation :type "Rotator Structure") (EquipmentHasSockets :type Boolean))
  (returns (EquipmentActor :type "/Game/Blueprints/CustomEquipmentBP Object Reference"))
  (locals (OverlayMaterialInstance :type "MaterialInstance Object Reference") (MeshScale :type "Vector Structure" :default (1.0 1.0 1.0)) (MeshRotation :type "Rotator Structure") (TrailScale :type "Vector Structure") (WeaponTrailMaterialInstance :type "MaterialInstance Object Reference" :default "/Script/Engine.MaterialInstanceConstant'/Game/Materials/CommonLootOutline_MI.CommonLootOutline_MI'") (Rarity :type "/Game/Blueprints/LootRarity Enum"))
  (bind _equipmentstaticmesh (`self.EquipmentStaticMesh`))
  (bind _equipmentstaticmesh_2 (`self.EquipmentStaticMesh`))
  (bind _weapontrail (`self.WeaponTrail`))
  (set `local.Rarity` EquipmentRarity)
  (set `local.TrailScale` TrailDisplayScale)
  (set `local.MeshScale` DisplayScale)
  (set `local.MeshRotation` DisplayRotation)
  (set `self.HasSockets` EquipmentHasSockets)
  (`StaticMeshComponent.SetStaticMesh` (`self.EquipmentStaticMesh`) EquipmentMesh)
  (switch `/Game/Blueprints/LootRarity` (`local.Rarity`)
    (:`NewEnumerator0`
      (set `local.OverlayMaterialInstance` "/Game/Materials/CommonLootOutline_MI.CommonLootOutline_MI"))
    (:`NewEnumerator1`
      (set `local.OverlayMaterialInstance` "/Game/Materials/UncommonLootOutline_MI.UncommonLootOutline_MI"))
    (:`NewEnumerator2`
      (set `local.OverlayMaterialInstance` "/Game/Materials/RareLootOutline_MI.RareLootOutline_MI"))
    (:`NewEnumerator3`
      (set `local.OverlayMaterialInstance` "/Game/Materials/EpicLootOutline_MI.EpicLootOutline_MI"))
    (:`NewEnumerator4`
      (set `local.OverlayMaterialInstance` "/Game/Materials/LegendaryLootOutline_MI.LegendaryLootOutline_MI"))
    (:`NewEnumerator5`
      (set `local.OverlayMaterialInstance` "/Game/Materials/MythicLootOutline_MI.MythicLootOutline_MI")))
  (`MeshComponent.SetOverlayMaterial` (`self.EquipmentStaticMesh`) (`local.OverlayMaterialInstance`))
  (`SceneComponent.SetRelativeScale3D` _equipmentstaticmesh_2 (`local.MeshScale`))
  (`SceneComponent.K2_SetRelativeRotation` _equipmentstaticmesh_2 (`local.MeshRotation`) false false)
  (if (`self.HasSockets`)
    (bind _output_get (set `self.BottomSocketPosition` (`SceneComponent.GetSocketLocation` _equipmentstaticmesh "BottomSocket")))
    (bind _output_get_2 (set `self.TopSocketPosition` (`SceneComponent.GetSocketLocation` _equipmentstaticmesh "TopSocket")))
    (bind _returnvalue (- _output_get_2 _output_get))
    (`FXSystemComponent.SetFloatParameter` _weapontrail "RibbonWidth" (`KismetMathLibrary.VSize` (* (`local.TrailScale`) _returnvalue)))
    (`SceneComponent.K2_SetWorldRotation` _weapontrail (`KismetMathLibrary.MakeRotFromZ` _returnvalue) false false)
    (`SceneComponent.K2_SetWorldLocation` _weapontrail (/ (+ _output_get _output_get_2) 2.0) false false)
    (bind _trailmaterialinstance (`self.GetWeaponTrailMaterialInstance` (`local.Rarity`)))
    (`NiagaraComponent.SetVariableMaterial` (`self.WeaponTrail`) "WeaponTrailMaterialInstance" _trailmaterialinstance))
  (return self))

(fn `UserConstructionScript`
  (locals (OverlayMaterialInstance :type "MaterialInstance Object Reference"))
  (`self.Update Equipment Attributes` (`self.CustomEquipmentStaticMesh`) (`self.EquipmentRarity`) (150.0 150.0 150.0) (150.0 150.0 150.0) (struct) true)
  (`self.SetTrailVisibility` false))