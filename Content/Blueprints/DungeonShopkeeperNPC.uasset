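; Dungeon shopkeeper NPC that switches the player into a shop view when they press OpenShop inside its trigger.
; ShopTrigger overlaps track whether the player is in range.
; Entering blends the camera to the NPC, hides the character and enables UI-only input with cursor; exiting reverses this, targeting the controller.
; No widget is created, and ShopOpen, which selects exit over enter, is never set here.
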(event `self.ShopTrigger.OnComponentBeginOverlap`
  (params (OverlappedComponent :type "PrimitiveComponent Object Reference") (OtherActor :type "Actor Object Reference") (OtherComp :type "PrimitiveComponent Object Reference") (OtherBodyIndex :type Integer) (bFromSweep :type Boolean) (SweepResult :type "HitResult Structure (by ref)"))
  (if (== OtherActor (`GameplayStatics.GetPlayerCharacter` 0))
    (set `self.PlayerInShopRange` true)
    (`KismetSystemLibrary.PrintString` "enter trigger")))

(event `self.ShopTrigger.OnComponentEndOverlap`
  (params (OverlappedComponent :type "PrimitiveComponent Object Reference") (OtherActor :type "Actor Object Reference") (OtherComp :type "PrimitiveComponent Object Reference") (OtherBodyIndex :type Integer))
  (if (== OtherActor (`GameplayStatics.GetPlayerCharacter` 0))
    (set `self.PlayerInShopRange` false)
    (`KismetSystemLibrary.PrintString` "exit trigger")))

(event `InputAction|OpenShop`
  (params (Key :type "Key Structure"))
  (:`Pressed`
    (`KismetSystemLibrary.PrintString` "shop pressed")
    (if (`self.ShopOpen`)
      (`KismetSystemLibrary.PrintString` "exit time")
      (`self.ExitShopMenu`)
      (elif (`self.PlayerInShopRange`)
        (`KismetSystemLibrary.PrintString` "enter time")
        (`self.EnterShopMenu`)))))

(fn `EnterShopMenu`
  (`PlayerController.SetViewTargetWithBlend` (`GameplayStatics.GetPlayerController` 0) self 1.0 "VTBlend_Linear" 0.0 false)
  (`WidgetBlueprintLibrary.SetInputMode_UIOnlyEx` (`GameplayStatics.GetPlayerController` 0) null)
  (set `PlayerController.bShowMouseCursor` true (`GameplayStatics.GetPlayerController` 0))
  (`self.SetActorHiddenInGame` (`GameplayStatics.GetPlayerCharacter` 0) true)
  (`KismetSystemLibrary.PrintString` "Enter shop menu"))

(fn `ExitShopMenu`
  (bind _returnvalue (`GameplayStatics.GetPlayerController` 0))
  (`PlayerController.SetViewTargetWithBlend` _returnvalue _returnvalue 1.0 "VTBlend_Linear" 0.0 false)
  (`WidgetBlueprintLibrary.SetInputMode_GameOnly` (`GameplayStatics.GetPlayerController` 0))
  (set `PlayerController.bShowMouseCursor` false (`GameplayStatics.GetPlayerController` 0))
  (`self.SetActorHiddenInGame` (`GameplayStatics.GetPlayerCharacter` 0) false)
  (`KismetSystemLibrary.PrintString` "Exit shop menu"))

(fn `UserConstructionScript`)