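; Torch is a configurable torch prop that can appear mounted or freestanding, lit or unlit.
; All setup runs in the construction script, which swaps between the two meshes and toggles the point light, orb and Niagara flame particles.
; When lit, one torch color drives the particle color, the orb's dynamic material and the light, with adjustable intensity and optional particles.
; The event graph holds no logic.
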(fn `UserConstructionScript`
  ;[1 1 1] Torch Mount/Unmount
  (`SceneComponent.SetVisibility` (`self.TorchMesh`) (not (`self.Mounted`)) false)
  (`SceneComponent.SetVisibility` (`self.MountedTorchMesh`) (`self.Mounted`) false)
  ;[1 1 1] Set Light Object Visibility
  (`SceneComponent.SetVisibility` (`self.TorchLight`) (`self.IsLit`) false)
  (`SceneComponent.SetVisibility` (`self.TorchOrb`) (`self.IsLit`) false)
  (`SceneComponent.SetVisibility` (`self.FlameParticles`) (`self.IsLit`) false)
  (if (`self.IsLit`)
    ;[1 1 1] Flame Particles
    (`NiagaraComponent.SetVariableLinearColor` (`self.FlameParticles`) "User.TorchFlameColor" (`self.TorchColor`))
    ;[1 1 1] Torch Orb
    (bind _returnvalue (`PrimitiveComponent.CreateDynamicMaterialInstance` (`self.TorchOrb`) 0 "/Game/Materials/TorchFlame.TorchFlame" "None"))
    (`MaterialInstanceDynamic.SetVectorParameterValue` _returnvalue "FlameColor" (`self.TorchColor`))
    ;[1 1 1] Torch Point Light
    (`LightComponent.SetLightColor` (`self.TorchLight`) (`self.TorchColor`) true)
    (`LightComponent.SetIntensity` (`self.TorchLight`) (`self.LightIntensity`))
    (`SceneComponent.SetVisibility` (`self.FlameParticles`) (`self.TorchHasParticles`) false)))