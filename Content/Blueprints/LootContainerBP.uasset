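; Loot container actor that shows an interact widget when the player is in range and, once opened, shakes and bursts out random loot.
; Construction script applies meshes and optional rarity outline and particle color.
; Tick moves both meshes along a spline, then BurstContainer spawns items from rarity class lists, with Mythic using the Legendary list.
; Items and container halves get physics impulses; the container switches to a dissolve material, then hides after a delay.
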(event `self.ReceiveBeginPlay`
  ;[1 1 1] Setup Initial Widget Visibility and Collision Ignores
  (`SceneComponent.SetVisibility` (`self.ContainerInteractWidget`) false false)
  (`PrimitiveComponent.IgnoreActorWhenMoving` (`self.MainContainerMesh`) self true)
  (`PrimitiveComponent.IgnoreActorWhenMoving` (`self.ContainerCoverMesh`) self true)
  ;[1 1 1] Grab Relative Mesh Locations for Mesh Shaking
  (set `self.InitialRelativeLocationContainer` (* (`SceneComponent.RelativeLocation` (`self.MainContainerMesh`)) (`SceneComponent.RelativeScale3D` (`self.BurstPoint`))))
  (set `self.InitialRelativeLocationContainerCover` (* (`SceneComponent.RelativeLocation` (`self.ContainerCoverMesh`)) (`SceneComponent.RelativeScale3D` (`self.BurstPoint`)))))

(event `self.ReceiveTick`
  (params (DeltaSeconds :type "Float (single-precision)"))
  (bind _shakespline (`self.ShakeSpline`))
  (bind _totalshakeduration (`self.TotalShakeDuration`))
  ;[1 1 1] Start Tracking Time after Container Opened
  (if (`self.ContainerOpenedAndShakeStarted`)
    (bind _output_get (set `self.CurrShakeTime` (+ DeltaSeconds (`self.CurrShakeTime`))))
    ;[1 1 1] Burst Container if CurrTime > TotalShake
    (if (> _output_get _totalshakeduration)
      (set `self.ShakeFinished` true)
      (`self.BurstContainer`)
      (if (not (`self.ContainerHidden`))
        ;[1 1 1] Hide Container After Shake is finished and hide delay has passed
        (if (>= (`self.CurrShakeTime`) (+ (`self.TotalShakeDuration`) (`self.PostBurstContainerHideDelay`)))
          (set `self.ContainerHidden` true)
          (`SceneComponent.SetVisibility` (`self.MainContainerMesh`) false false)
          (`SceneComponent.SetVisibility` (`self.ContainerCoverMesh`) false false)))
      (else
        (bind _returnvalue (`KismetMathLibrary.TransformLocation` (`SceneComponent.K2_GetComponentToWorld` (`self.BurstPoint`)) (`KismetMathLibrary.TransformLocation` (`SplineComponent.GetTransformAtDistanceAlongSpline` _shakespline (* (`SplineComponent.GetSplineLength` _shakespline) (`KismetMathLibrary.FMin` (/ _output_get _totalshakeduration) 1.0)) "Local" false))))
        ;[1 1 1] Set Location of Container Meshes
        (`SceneComponent.K2_SetWorldLocation` (`self.MainContainerMesh`) (+ _returnvalue (`self.InitialRelativeLocationContainer`)) false false)
        (`SceneComponent.K2_SetWorldLocation` (`self.ContainerCoverMesh`) (+ _returnvalue (`self.InitialRelativeLocationContainerCover`)) false false)))))

(event `self.ContainerInteractionCollisionSphere.OnComponentBeginOverlap`
  (params (OverlappedComponent :type "PrimitiveComponent Object Reference") (OtherActor :type "Actor Object Reference") (OtherComp :type "PrimitiveComponent Object Reference") (OtherBodyIndex :type Integer) (bFromSweep :type Boolean) (SweepResult :type "HitResult Structure (by ref)"))
  (if (== OtherActor (`GameplayStatics.GetPlayerCharacter` 0))
    (set `self.PlayerWithinInteractionRange` true)
    (`self.UpdateContainerWidgetVisibility`)))

(event `self.ContainerInteractionCollisionSphere.OnComponentEndOverlap`
  (params (OverlappedComponent :type "PrimitiveComponent Object Reference") (OtherActor :type "Actor Object Reference") (OtherComp :type "PrimitiveComponent Object Reference") (OtherBodyIndex :type Integer))
  (if (== OtherActor (`GameplayStatics.GetPlayerCharacter` 0))
    (set `self.PlayerWithinInteractionRange` false)
    (`self.UpdateContainerWidgetVisibility`)))

(fn `BurstContainer`
  (bind _maincontainermesh (`self.MainContainerMesh`))
  (bind _containercovermesh (`self.ContainerCoverMesh`))
  (bind _returnvalue (* (`KismetMathLibrary.Normal` (+ (* (`KismetMathLibrary.RandomUnitVector`) (`self.ContainerBurstRotationIntensity`)) (`SceneComponent.GetForwardVector` (`self.BurstDirection`)))) (* (`self.ContainerBurstForce`) 1000.0)))
  (if (not (`self.ContainerIsBurst`))
    (`KismetSystemLibrary.PrintString` "Bursting container")
    (`GameplayStatics.PlaySoundAtLocation` (`self.ContainerOpenSound`) (`SceneComponent.K2_GetComponentLocation` (`self.BurstPoint`)) (struct) 1.0 1.0 0.0 null null null null)
    (`ActorComponent.Deactivate` (`self.BurstParticle`))
    (set `self.ContainerIsBurst` true)
    (`self.BurstItems`)
    (`PrimitiveComponent.SetSimulatePhysics` _containercovermesh true)
    (`PrimitiveComponent.AddForce` _containercovermesh _returnvalue "None" true)
    (`PrimitiveComponent.AddTorqueInDegrees` _containercovermesh (* (`KismetMathLibrary.RandomUnitVector`) (* (`self.ContainerBurstRotationIntensity`) 20000000.0)) "None" false)
    (`PrimitiveComponent.SetSimulatePhysics` _maincontainermesh true)
    (`PrimitiveComponent.AddForce` _maincontainermesh (* _returnvalue -1.0) "None" true)
    (`PrimitiveComponent.AddTorqueInDegrees` _maincontainermesh (* (`KismetMathLibrary.RandomUnitVector`) (* (`self.ContainerBurstRotationIntensity`) 20000000.0)) "None" false)
    (`PrimitiveComponent.SetMaterial` (`self.MainContainerMesh`) 0 "/Game/Materials/DissolveInstance.DissolveInstance")
    (`PrimitiveComponent.SetMaterial` (`self.ContainerCoverMesh`) 0 "/Game/Materials/DissolveInstance.DissolveInstance")))

(fn `BurstItems`
  (bind _lootitems (`self.GenerateLootItems`))
  (for _array_element _lootitems
    (`self.K2_SetActorLocation` _array_element (`SceneComponent.K2_GetComponentLocation` (`self.BurstPoint`)) false false)
    (bind _lootmesh (`/Game/Blueprints/LootBP.LootMesh` _array_element))
    (`PrimitiveComponent.SetSimulatePhysics` _lootmesh true)
    (`PrimitiveComponent.AddForce` _lootmesh (* (`KismetMathLibrary.Normal` (+ (* (`KismetMathLibrary.RandomUnitVector`) (`self.ItemBurstRotationIntensity`)) (`SceneComponent.GetForwardVector` (`self.BurstDirection`)))) (* (`self.ItemBurstForce`) 1000.0)) "None" true)
    (`PrimitiveComponent.AddTorqueInDegrees` _lootmesh (* (`KismetMathLibrary.RandomUnitVector`) (* (`self.ItemBurstRotationIntensity`) 20000000.0)) "None" false)))

(fn `GenerateLootItems`
  (returns (LootItems :type "Array of /Game/Blueprints/LootBP Object Reference"))
  (locals (LootItemActors :type "Array of /Game/Blueprints/LootBP Object Reference") (CommonLootClassRefs :type "Array of /Game/Blueprints/LootBP Class Reference") (UncommonLootClassRefs :type "Array of /Game/Blueprints/LootBP Class Reference") (RareLootClassRefs :type "Array of /Game/Blueprints/LootBP Class Reference") (EpicLootClassRefs :type "Array of /Game/Blueprints/LootBP Class Reference") (LegendaryLootClassRefs :type "Array of /Game/Blueprints/LootBP Class Reference") (CurrentRarityClassRefs :type "Array of /Game/Blueprints/LootBP Class Reference"))
  (switch `/Game/Blueprints/LootRarity` (`self.ContainerRarity`)
    (:`NewEnumerator0`
      (set `local.CurrentRarityClassRefs` (`local.CommonLootClassRefs`)))
    (:`NewEnumerator1`
      (set `local.CurrentRarityClassRefs` (`local.UncommonLootClassRefs`)))
    (:`NewEnumerator2`
      (set `local.CurrentRarityClassRefs` (`local.RareLootClassRefs`)))
    (:`NewEnumerator3`
      (set `local.CurrentRarityClassRefs` (`local.EpicLootClassRefs`)))
    (:`NewEnumerator4`
      (set `local.CurrentRarityClassRefs` (`local.LegendaryLootClassRefs`)))
    (:`NewEnumerator5`
      (set `local.CurrentRarityClassRefs` (`local.LegendaryLootClassRefs`))))
  (for _ (range 1 (+ (`self.ItemCount`) 1))
    (bind _returnvalue (`|SpawnActorFromClass` (`KismetArrayLibrary.Array_Random` (`local.CurrentRarityClassRefs`)) (`KismetMathLibrary.MakeTransform` (`SceneComponent.K2_GetComponentLocation` (`self.BurstPoint`))) "AlwaysSpawn" "MultiplyWithRoot" null null))
    (`KismetArrayLibrary.Array_Add` (`local.LootItemActors`) _returnvalue))
  (return (`local.LootItemActors`)))

(fn `GetRandomLootClassForRarity`
  (params (LootRarity :type "/Game/Blueprints/LootRarity Enum" :default "NewEnumerator0"))
  (returns (NewParam :type "/Game/Blueprints/LootBP Class Reference"))
  (switch `/Game/Blueprints/LootRarity` LootRarity))

(fn `GetRarityMaterialColor`
  (returns (`Rarity Material Color` :type "LinearColor Structure"))
  (locals (CommonRarityColor :type "LinearColor Structure" :default (struct :`R` 0.94902 :`G` 1.0 :`B` 0.956863 :`A` 1.0)) (UncommonRarityColor :type "LinearColor Structure" :default (struct :`R` 0.007843 :`G` 1.0 :`B` 0.156863 :`A` 1.0)) (RareRarityColor :type "LinearColor Structure" :default (struct :`R` 0.84 :`G` 3.63 :`B` 100.0 :`A` 1.0)) (EpicRarityColor :type "LinearColor Structure" :default (struct :`R` 0.937255 :`B` 1.0 :`A` 1.0)) (LegendaryRarityColor :type "LinearColor Structure" :default (struct :`R` 10.0 :`G` 5.2 :`A` 1.0)) (MythicRarityColor :type "LinearColor Structure" :default (struct :`R` 10.0 :`G` 0.286275 :`A` 1.0)))
  (switch `/Game/Blueprints/LootRarity` (`self.ContainerRarity`)
    (:`NewEnumerator0`
      (return (`local.CommonRarityColor`)))
    (:`NewEnumerator1`
      (return (`local.UncommonRarityColor`)))
    (:`NewEnumerator2`
      (return (`local.RareRarityColor`)))
    (:`NewEnumerator3`
      (return (`local.EpicRarityColor`)))
    (:`NewEnumerator4`
      (return (`local.LegendaryRarityColor`)))
    (:`NewEnumerator5`
      (return (`local.MythicRarityColor`)))))

(fn `PlayerOpenContainer`
  (if (and (not (`self.ContainerOpenedAndShakeStarted`)) (`self.PlayerWithinInteractionRange`))
    (set `self.ContainerOpenedAndShakeStarted` true)
    (`self.UpdateContainerWidgetVisibility`)
    (`ActorComponent.Activate` (`self.BurstParticle`) false)
    (`GameplayStatics.PlaySoundAtLocation` (`self.ContainerBurstingSound`) (`SceneComponent.K2_GetComponentLocation` (`self.BurstPoint`)) (struct) 1.0 1.0 0.0 null null null null)))

(fn `UpdateContainerWidgetVisibility`
  ;[1 1 1] Hide Widget if Container Opened or Out of Range
  (`SceneComponent.SetVisibility` (`self.ContainerInteractWidget`) (and (not (`self.ContainerOpenedAndShakeStarted`)) (`self.PlayerWithinInteractionRange`)) false))

(fn `UserConstructionScript`
  (`StaticMeshComponent.SetStaticMesh` (`self.MainContainerMesh`) (`self.CustomContainerMesh`))
  (`StaticMeshComponent.SetStaticMesh` (`self.ContainerCoverMesh`) (`self.CustomContairerCoverMesh`))
  (if (`self.ContainerHasRarityGlow`)
    (switch `/Game/Blueprints/LootRarity` (`self.ContainerRarity`)
      (:`NewEnumerator0`
        (set `self.OverlayMaterialInstance` "/Game/Materials/CommonLootOutline_MI.CommonLootOutline_MI"))
      (:`NewEnumerator1`
        (set `self.OverlayMaterialInstance` "/Game/Materials/UncommonLootOutline_MI.UncommonLootOutline_MI"))
      (:`NewEnumerator2`
        (set `self.OverlayMaterialInstance` "/Game/Materials/RareLootOutline_MI.RareLootOutline_MI"))
      (:`NewEnumerator3`
        (set `self.OverlayMaterialInstance` "/Game/Materials/EpicLootOutline_MI.EpicLootOutline_MI"))
      (:`NewEnumerator4`
        (set `self.OverlayMaterialInstance` "/Game/Materials/LegendaryLootOutline_MI.LegendaryLootOutline_MI"))
      (:`NewEnumerator5`
        (set `self.OverlayMaterialInstance` "/Game/Materials/MythicLootOutline_MI.MythicLootOutline_MI")))
    (`MeshComponent.SetOverlayMaterial` (`self.MainContainerMesh`) (`self.OverlayMaterialInstance`))
    (`MeshComponent.SetOverlayMaterial` (`self.ContainerCoverMesh`) (`self.OverlayMaterialInstance`))
    (bind _rarity_material_color (`self.GetRarityMaterialColor`))
    (`NiagaraComponent.SetVariableLinearColor` (`self.BurstParticle`) "User.BurstParticleColor" _rarity_material_color)
    (`SphereComponent.SetSphereRadius` (`self.ContainerInteractionCollisionSphere`) (`self.CollisionRadius`) true)))